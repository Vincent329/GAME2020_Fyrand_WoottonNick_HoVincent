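; Player-driven pickup vehicle with a camera-aimed mounted gun that fires BP_Bullet, a flip reset, HUD and pause menu.
; Axis inputs drive VehicleMovement and the camera, while G is a test key that lowers FullHealth.
; Construction caches all CharSplinePath actors; Tick polls their Collision flags, then teleports the truck along the touched spline at fixed yaw until near its end, zeroing movement velocity each step.
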(event EventTick
  (params (DeltaSeconds :type Float%20%28single-precision%29))
  (bind _mesh (Variables|Character|GetMesh))
  (bind _returnvalue (Transformation|GetWorldLocation _mesh))
  ;[1 0.3281 0] check for collision with a spline
  (if (Variables|Default|GetMovingOnSpline)
    (Development|PrintString (Utilities|String|Append (Utilities|String|Append (Utilities|String|Append "X: " (Utilities|String|ToString(Float) (.X (Math|Vector|BreakVector (* (Variables|Default|GetSplineVelocity) (Variables|Default|GetSplineConstSpeed)))))) (Utilities|String|Append "  |  Y: " (Utilities|String|ToString(Float) (.Y (Math|Vector|BreakVector (* (Variables|Default|GetSplineVelocity) (Variables|Default|GetSplineConstSpeed))))))) (Utilities|String|Append (Utilities|String|Append "  |  X: " (Utilities|String|ToString(Float) (.X (Math|Vector|BreakVector (+ (* (Variables|Default|GetSplineVelocity) (Variables|Default|GetSplineConstSpeed)) _returnvalue))))) (Utilities|String|Append "  |  Y: " (Utilities|String|ToString(Float) (.Y (Math|Vector|BreakVector (+ (* (Variables|Default|GetSplineVelocity) (Variables|Default|GetSplineConstSpeed)) _returnvalue))))))) true true "(R=0.000000,G=0.660000,B=1.000000,A=1.000000)" 0.0005)
    ;[0.1016 0 1] TRUE: continue to teleport the vehicle along the spline
    ; FALSE: Exit spline if vehicle has hit the end
    (if (and (< (Math|Float|Absolute(Float) (.Y (Math|Vector|BreakVector (- (Spline|GetLocationatSplinePoint (Variables|Default|GetSplineRef) (- (Spline|GetNumberOfSplinePoints (Variables|Default|GetSplineRef)) 1) "World") _returnvalue)))) (Math|Float|Absolute(Float) (.Y (Math|Vector|BreakVector (* (* (Variables|Default|GetSplineVelocity) (Variables|Default|GetSplineConstSpeed)) 4))))) (< (Math|Float|Absolute(Float) (.X (Math|Vector|BreakVector (- (Spline|GetLocationatSplinePoint (Variables|Default|GetSplineRef) (- (Spline|GetNumberOfSplinePoints (Variables|Default|GetSplineRef)) 1) "World") _returnvalue)))) (Math|Float|Absolute(Float) (.X (Math|Vector|BreakVector (* (* (Variables|Default|GetSplineVelocity) (Variables|Default|GetSplineConstSpeed)) 4))))))
      (Variables|Default|SetMovingOnSpline false)
      (Variables|Default|SetsplineCounter 0)
      (Variables|Default|SetSplineRef 0)
      (Variables|Default|SetSplineVelocity "0, 0, 0")
      (Development|PrintString "end")
      (else
        (Transformation|Teleport (Spline|FindLocationClosesttoWorldLocation (Variables|Default|GetSplineRef) (+ (* (Variables|Default|GetSplineVelocity) (Variables|Default|GetSplineConstSpeed)) _returnvalue) "World") (Math|Rotator|MakeRotator 0.0 0.0 (Variables|Default|GetStartYaw)))
        (Variables|/Script/Engine.MovementComponent|SetVelocity (Variables|Default|GetVehicleMovement) "0, 0, 0")))
    (else
      (for _array_element (Variables|Default|GetCharSplineArray)
        ;[0 1 0.8359] Start of spline movement
        (if (Variables|/Game/CharSplinePath.CharSplinePath_C|GetCollision _array_element)
          (Variables|Default|SetStartYaw (.Yaw (Math|Rotator|BreakRotator (Transformation|GetWorldRotation (Variables|Character|GetMesh)))))
          (Variables|Default|SetSplineRef (Variables|/Game/CharSplinePath.CharSplinePath_C|GetSpline _array_element))
          (Variables|Default|SetMovingOnSpline true)
          (Variables|Default|SetSplineVelocity (* (- (Spline|GetLocationatSplinePoint (Variables|Default|GetSplineRef) 0 "World") (Transformation|GetWorldLocation (Variables|Character|GetMesh))) (Utilities|Time|GetWorldDeltaSeconds)))
          (Development|PrintString "start"))))))

(event EventBeginPlay
  ;[1 0 0.3984] UI Display
  (bind _returnvalue (UserInterface|CreateWidget "/Game/MenuAssets/UserInterface.UserInterface_C"))
  (UserInterface|Viewport|AddtoViewport _returnvalue 0))

(event Input|ActionEvents|InputActionResetVehicle
  (params (Key :type Key%20Structure :default "None"))
  (bind _mesh (Variables|Character|GetMesh))
  (bind _returnvalue (Transformation|GetWorldLocation _mesh))
  (bind (_x _y _z) (Math|Vector|BreakVector _returnvalue))
  ;[0.3828 1 0] Spacebar -> Flip Vehicle
  (:Pressed
    (Transformation|Teleport (Math|Vector|MakeVector _x _y (+ _z 8e+01)) (Math|Rotator|MakeRotator 0.0 0.0 (.Yaw (Math|Rotator|BreakRotator (Transformation|GetWorldRotation _mesh)))))
    (Variables|/Script/Engine.MovementComponent|SetVelocity (Variables|Default|GetVehicleMovement) "0, 0, 0")))

(event Input|ActionEvents|InputActionFire
  (params (Key :type Key%20Structure :default "None"))
  (bind _sm_ka47_x (Variables|Default|GetSM_KA47_X))
  (bind _mesh (Variables|Character|GetMesh))
  (bind _returnvalue (Transformation|GetWorldLocation _mesh))
  (bind _returnvalue_2 (Transformation|GetWorldRotation _sm_ka47_x))
  (bind (_x _y _z) (Math|Vector|BreakVector _returnvalue))
  ;[0 0.1328 1] Fire bullets
  (:Pressed
    (bind _returnvalue_3 (Game|SpawnActorfromClass "/Game/BP_Bullet.BP_Bullet_C" (Math|Transform|MakeTransform (Math|Vector|MakeVector _x _y (+ _z 1.1e+02)) (Transformation|GetWorldRotation _mesh) "0.100000,0.100000,0.100000") "Undefined" 0 0))
    (Variables|/Game/BP_Bullet.BP_Bullet_C|SetVelocity _returnvalue_3 (Math|Rotator|GetRotationXVector _returnvalue_2))
    (Transformation|SetActorRotation _returnvalue_3 _returnvalue_2)))

(event Input|ActionEvents|InputActionPause
  (params (Key :type Key%20Structure :default "None"))
  ;[0.125 0 1] Pause the Game
  (:Pressed
    (CallFunction|PauseGame)))

(event Input|AxisEvents|InputAxisMouseX
  (params (AxisValue :type Float%20%28single-precision%29))
  ;[1 0 0.1641] vehicle camera control
  (Pawn|Input|AddControllerYawInput AxisValue)
  (Transformation|SetWorldRotation (Variables|Default|GetSM_KA47_X) (Transformation|GetSocketRotation (Variables|Components|GetCamera) "None") false false))

(event Input|AxisEvents|InputAxisMouseY
  (params (AxisValue :type Float%20%28single-precision%29))
  ;[1 0 0.1641] vehicle camera control
  (Pawn|Input|AddControllerPitchInput (* AxisValue -1.0)))

(event Input|AxisEvents|InputAxisForward
  (params (AxisValue :type Float%20%28single-precision%29))
  ;[0 1 0.5781] vehicle movement
  (Class|WheeledVehicleMovementComponent|SetThrottleInput (Variables|Default|GetVehicleMovement) AxisValue))

(event Input|AxisEvents|InputAxisTurn
  (params (AxisValue :type Float%20%28single-precision%29))
  ;[0 1 0.5781] vehicle movement
  (Class|WheeledVehicleMovementComponent|SetSteeringInput (Variables|Default|GetVehicleMovement) AxisValue))

(event Input|KeyboardEvents|G
  (params (Key :type Key%20Structure :default "None"))
  ;[0.9688 1 0] Damage Test
  (:Pressed
    (Variables|Default|SetFullHealth (- (Variables|Default|GetFullHealth) 5.0))))

(fn ConstructionScript
  (bind _outactors (Actor|GetAllActorsOfClass "/Game/CharSplinePath.CharSplinePath_C"))
  (Variables|Default|SetCharSplineArray _outactors)
  (Variables|Default|SetCurrentHealth (Variables|Default|GetFullHealth)))

(fn PauseGame
  (Game|SetGamePaused true)
  (Utilities|IsValid (Variables|Default|GetPauseMenu)
    (:Is%20Valid
      _)
    (:Is%20Not%20Valid
      (bind _returnvalue (UserInterface|CreateWidget "/Game/MenuAssets/PauseMenu.PauseMenu_C" (Game|GetPlayerController 0)))
      (Variables|Default|SetPauseMenu _returnvalue)))
  (UserInterface|Viewport|AddtoViewport (Variables|Default|GetPauseMenu) 0)
  (Input|SetInputModeUIOnly (Game|GetPlayerController 0) (Variables|Default|GetPauseMenu) "DoNotLock")
  (Variables|/Script/Engine.PlayerController|SetbShowMouseCursor (Game|GetPlayerController 0) true))

(fn UnpauseGame
  (bind _returnvalue (Game|GetPlayerController 0))
  (Game|SetGamePaused false)
  (Viewport|RemoveAllWidgets)
  (Input|SetInputModeGameOnly _returnvalue)
  (Variables|/Script/Engine.PlayerController|SetbShowMouseCursor _returnvalue false)
  (bind _returnvalue_2 (UserInterface|CreateWidget "/Game/MenuAssets/UserInterface.UserInterface_C"))
  (UserInterface|Viewport|AddtoViewport _returnvalue_2 0))

(fn CheckforRoll
  (params (inFloat :type Float%20%28single-precision%29))
  (if (or (> inFloat 8e+01) (< inFloat -8e+01))
    (Development|PrintString "Rolling")
    (return (- inFloat (* (+ (Math|Conversions|ToFloat(Boolean) (> inFloat 0.0)) (* (Math|Conversions|ToFloat(Boolean) (< inFloat 0.0)) -1.0)) (Variables|Default|GetRollSpeed))))
    (else
      (return inFloat))))